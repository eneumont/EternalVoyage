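; Automatic sliding door that lowers while a player or VR pawn is inside its trigger box.
; Box begin overlap accepts BP_Player or VRPawn and moves the door mesh and its back piece down together over one second.
; End overlap returns both to a zero relative location, with the back piece keeping its half-turn rotation in both moves.
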(event OnComponentEndOverlap(Box)
  (params (OverlappedComponent :type Primitive%20Component%20Object%20Reference) (OtherActor :type Actor%20Object%20Reference) (OtherComp :type Primitive%20Component%20Object%20Reference) (OtherBodyIndex :type Integer))
  (Utilities|Casting|CastToBP_Player OtherActor
    (:then
      _)
    (:CastFailed
      (Utilities|Casting|CastToVRPawn OtherActor)))
  (Utilities|FlowControl|Sequence
    (:then_0
      (Components|MoveComponentTo (Variables|Default|GetStaticMesh) "0, 0, 0" "0, 0, 0" false false 1.0 false))
    (:then_1
      (Components|MoveComponentTo (Variables|Default|GetTheFuckinBack) "0, 0, 0" "0.000000,-180.000000,0.000000" false false 1.0 false))))

(event OnComponentBeginOverlap(Box)
  (params (OverlappedComponent :type Primitive%20Component%20Object%20Reference) (OtherActor :type Actor%20Object%20Reference) (OtherComp :type Primitive%20Component%20Object%20Reference) (OtherBodyIndex :type Integer) (bFromSweep :type Boolean) (SweepResult :type Hit%20Result%20Structure%20%28by%20ref%29))
  (Utilities|Casting|CastToBP_Player OtherActor
    (:then
      _)
    (:CastFailed
      (Utilities|Casting|CastToVRPawn OtherActor)))
  (Utilities|FlowControl|Sequence
    (:then_0
      (Components|MoveComponentTo (Variables|Default|GetTheFuckinBack) "0.000000,0.000000,-656.000000" "0.000000,-180.000000,0.000000" false false 1.0 false))
    (:then_1
      (Components|MoveComponentTo (Variables|Default|GetStaticMesh) "0.000000,0.000000,-656.000000" "0, 0, 0" false false 1.0 false))))

(event EventBeginPlay)

(event Collision|EventActorBeginOverlap
  (params (OtherActor :type Actor%20Object%20Reference)))

(event EventTick
  (params (DeltaSeconds :type Float%20%28single-precision%29)))

(fn ConstructionScript)