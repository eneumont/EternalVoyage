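; BP_TaskSpawnerReactor is the reactor variant of a task spawner, with its core behavior left to its parent class.
; On BeginPlay it casts the game instance to BP_GameInstance, copies ReactorScore into its Score variable, then calls the parent BeginPlay.
; If the cast fails, the parent BeginPlay is not called.
; Overlap and Tick are disabled stubs, and the construction script only calls the parent.
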(event EventBeginPlay
  (bind _asbp_game_instance (Utilities|Casting|CastToBP_GameInstance (Game|GetGameInstance)))
  (Variables|Default|SetScore (Variables|/Game/GAME/Blueprints/BP_GameInstance.BP_GameInstance_C|GetReactorScore _asbp_game_instance))
  (|CallParentFunction))

(event Collision|EventActorBeginOverlap
  (params (OtherActor :type Actor%20Object%20Reference))
  (|CallParentFunction OtherActor) ; This node is disabled and will not be called.\nDrag off pins to build functionality.
)

(event EventTick
  (params (DeltaSeconds :type Float%20%28single-precision%29))
  (|CallParentFunction DeltaSeconds) ; This node is disabled and will not be called.\nDrag off pins to build functionality.
)

(fn ConstructionScript
  (|CallParentFunction))