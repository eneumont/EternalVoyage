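; BP_TaskManager runs the day loop and chooses the game's ending.
; On construction and BeginPlay it reads the day count from BP_GameInstance, gathers all task actors and creates the task manager widget.
; NextDay saves the day, crew and Tree, Pilot and Reactor spawner scores to the game instance, then reloads FinalMap.
; After the last day, it totals all spawner scores to open the good or bad ending level.
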(event EventBeginPlay
  (CallFunction|CreateUI))

(event Collision|EventActorBeginOverlap
  (params (OtherActor :type Actor%20Object%20Reference)))

(event EventTick
  (params (DeltaSeconds :type Float%20%28single-precision%29)))

(fn ConstructionScript
  (CallFunction|CreateUI))

(fn NextDay
  (bind _returnvalue (Game|GetGameInstance))
  (if (< (Variables|Default|GetTotalDays) (Variables|Default|GetMaxDays))
    (bind _result (Math|Integer|IncrementInt (Variables|Default|GetTotalDays))
      (:%20%20
        (bind _output_get (Variables|Default|SetTotalDays _result))
        (bind _asbp_game_instance (Utilities|Casting|CastToBP_GameInstance (Game|GetGameInstance)))
        (Variables|/Game/GAME/Blueprints/BP_GameInstance.BP_GameInstance_C|SetDays _asbp_game_instance _output_get)
        (bind _asbp_player (Utilities|Casting|CastToBP_Player (Game|Player|GetPlayerPawn 0)))
        (Variables|/Game/GAME/Blueprints/BP_GameInstance.BP_GameInstance_C|SetCrew _asbp_game_instance (Variables|/Game/GAME/Blueprints/Player_Blueprints/BP_Player.BP_Player_C|GetCrew _asbp_player))
        (Utilities|FlowControl|Sequence
          (:then_0
            (bind _returnvalue_2 (Actor|GetActorOfClass "/Game/GAME/Blueprints/Task_Blueprints/BP_TaskSpawnerTree.BP_TaskSpawnerTree_C"))
            (bind _asbp_game_instance_2 (Utilities|Casting|CastToBP_GameInstance _returnvalue))
            (Variables|/Game/GAME/Blueprints/BP_GameInstance.BP_GameInstance_C|SetTreeScore _asbp_game_instance_2 (Variables|/Game/GAME/Blueprints/Task_Blueprints/BP_TaskSpawnerBase.BP_TaskSpawnerBase_C|GetScore _returnvalue_2)))
          (:then_1
            (bind _returnvalue_3 (Actor|GetActorOfClass "/Game/GAME/Blueprints/Task_Blueprints/BP_TaskSpawnerPilot.BP_TaskSpawnerPilot_C"))
            (bind _asbp_game_instance_3 (Utilities|Casting|CastToBP_GameInstance _returnvalue))
            (Variables|/Game/GAME/Blueprints/BP_GameInstance.BP_GameInstance_C|SetPilotScore _asbp_game_instance_3 (Variables|/Game/GAME/Blueprints/Task_Blueprints/BP_TaskSpawnerBase.BP_TaskSpawnerBase_C|GetScore _returnvalue_3)))
          (:then_2
            (bind _returnvalue_4 (Actor|GetActorOfClass "/Game/GAME/Blueprints/Task_Blueprints/BP_TaskSpawnerReactor.BP_TaskSpawnerReactor_C"))
            (bind _asbp_game_instance_4 (Utilities|Casting|CastToBP_GameInstance _returnvalue))
            (Variables|/Game/GAME/Blueprints/BP_GameInstance.BP_GameInstance_C|SetReactorScore _asbp_game_instance_4 (Variables|/Game/GAME/Blueprints/Task_Blueprints/BP_TaskSpawnerBase.BP_TaskSpawnerBase_C|GetScore _returnvalue_4)))
          (:then_3
            (bind _asbp_game_instance_5 (Utilities|Casting|CastToBP_GameInstance (Game|GetGameInstance)))
            (Variables|/Game/GAME/Blueprints/BP_GameInstance.BP_GameInstance_C|SetLoop _asbp_game_instance_5 true)
            (Game|OpenLevel(byName) "FinalMap")))))
    (else
      (CallFunction|GetEnding))))

(fn GetEnding
  (bind _outactors (Actor|GetAllActorsOfClass "/Game/GAME/Blueprints/Task_Blueprints/BP_TaskSpawnerBase.BP_TaskSpawnerBase_C"))
  (for _array_element _outactors
    (Variables|Default|SetScore (+ (Variables|/Game/GAME/Blueprints/Task_Blueprints/BP_TaskSpawnerBase.BP_TaskSpawnerBase_C|GetScore _array_element) (Variables|Default|GetScore))))
  (if (>= (Variables|Default|GetScore) 12)
    (Game|OpenLevel(byName) "GoodEnding")
    (else
      (Game|OpenLevel(byName) "BadEnding"))))

(fn CreateUI
  (bind _asbp_game_instance (Utilities|Casting|CastToBP_GameInstance (Game|GetGameInstance)))
  (Variables|Default|SetTotalDays (Variables|/Game/GAME/Blueprints/BP_GameInstance.BP_GameInstance_C|GetDays _asbp_game_instance))
  (bind _outactors (Actor|GetAllActorsOfClass "/Game/GAME/Blueprints/Task_Blueprints/BP_TaskBase.BP_TaskBase_C"))
  (Variables|Default|SetTasks _outactors)
  (UserInterface|CreateWidget "/Game/GAME/UI/TaskUI/WB_TaskManager.WB_TaskManager_C")
  (return 0))