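; Base actor for an interactable task that crew players complete and non-crew players sabotage.
; Player overlap enables input and shows a WB_DoThing prompt if that role's action is not yet done; leaving removes both.
; DoTask and DoSabotage set their flags and raise or lower the score on SpawnerRef, which stays frozen once it equals either limit.
; Done only prints an already-done message.
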(event EventBeginPlay)

(event Collision|EventActorBeginOverlap
  (params (OtherActor :type Actor%20Object%20Reference))
  (bind _asbp_player (Utilities|Casting|CastToBP_Player OtherActor))
  (Input|EnableInput (Game|GetPlayerController 0))
  (if (Variables|/Game/GAME/Blueprints/Player_Blueprints/BP_Player.BP_Player_C|GetCrew _asbp_player)
    (if (not (Variables|Default|GetComplete?))
      ;[1 1 1] display a widget
      (bind _returnvalue (UserInterface|CreateWidget "/Game/GAME/UI/TaskUI/WB_DoThing.WB_DoThing_C" :!label _label))
      (UserInterface|Viewport|AddtoViewport _returnvalue 0))
    (elif (not (Variables|Default|GetSabotage?))
      (goto _label))))

(event EventTick
  (params (DeltaSeconds :type Float%20%28single-precision%29)))

(event Collision|EventActorEndOverlap
  (params (OtherActor :type Actor%20Object%20Reference))
  (Utilities|Casting|CastToBP_Player OtherActor)
  (Input|DisableInput (Game|GetPlayerController 0))
  (Widget|RemovefromParent (stale Collision|EventActorBeginOverlap _returnvalue)))

(fn ConstructionScript)

(fn DoTask
  (bind _spawnerref (Variables|Default|GetSpawnerRef))
  (Variables|Default|SetComplete? true)
  (if (not (or (== (Variables|/Game/GAME/Blueprints/Task_Blueprints/BP_TaskSpawnerBase.BP_TaskSpawnerBase_C|GetScore (Variables|Default|GetSpawnerRef)) 6) (== (Variables|/Game/GAME/Blueprints/Task_Blueprints/BP_TaskSpawnerBase.BP_TaskSpawnerBase_C|GetScore (Variables|Default|GetSpawnerRef)) 0)))
    (bind _result (Math|Integer|IncrementInt (Variables|/Game/GAME/Blueprints/Task_Blueprints/BP_TaskSpawnerBase.BP_TaskSpawnerBase_C|GetScore _spawnerref))
      (:%20%20
        (Variables|/Game/GAME/Blueprints/Task_Blueprints/BP_TaskSpawnerBase.BP_TaskSpawnerBase_C|SetScore _spawnerref _result)))))

(fn DoSabotage
  (bind _spawnerref (Variables|Default|GetSpawnerRef))
  (Variables|Default|SetSabotage? true)
  (if (not (or (== (Variables|/Game/GAME/Blueprints/Task_Blueprints/BP_TaskSpawnerBase.BP_TaskSpawnerBase_C|GetScore (Variables|Default|GetSpawnerRef)) 6) (== (Variables|/Game/GAME/Blueprints/Task_Blueprints/BP_TaskSpawnerBase.BP_TaskSpawnerBase_C|GetScore (Variables|Default|GetSpawnerRef)) 0)))
    (bind _result (Math|Integer|DecrementInt (Variables|/Game/GAME/Blueprints/Task_Blueprints/BP_TaskSpawnerBase.BP_TaskSpawnerBase_C|GetScore _spawnerref))
      (:%20%20
        (Variables|/Game/GAME/Blueprints/Task_Blueprints/BP_TaskSpawnerBase.BP_TaskSpawnerBase_C|SetScore _spawnerref _result)))))

(fn Done
  (Development|PrintString "already done..."))